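; Rat NPC character blueprint with health, death handling and player detection.
; Damage lowers and prints Health; at zero it plays the death animation, deactivates movement and destroys the actor after a delay.
; The delayed mesh stop is timed later than the destroy.
; PawnSensing sets the AI controller's "HasSenPlayer?" blackboard flag when it sees the third-person player character, and nothing here clears it.
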(event OnSeePawn(PawnSensing)
  (params (Pawn :type Pawn%20Object%20Reference))
  (Utilities|Casting|CastToBP_ThirdPersonCharacter Pawn)
  (AI|Components|Blackboard|SetValueasBool (AI|GetBlackboard (AI|GetAIController self)) (Utilities|Name|MakeLiteralName "HasSenPlayer?") true))

(event EventBeginPlay)

(event Collision|EventActorBeginOverlap
  (params (OtherActor :type Actor%20Object%20Reference)))

(event EventTick
  (params (DeltaSeconds :type Float%20%28single-precision%29)))

(event EventDamage
  (params (Damage :type Float%20%28double-precision%29))
  (bind _output_get (Variables|RatHealt|SetHealth (Math|Float|Max(Float) (- (Variables|RatHealt|GetHealth) Damage) 0.0)))
  (Development|PrintString (Utilities|String|ToString(Float) _output_get))
  (if (== (Variables|RatHealt|GetHealth) 0.0)
    (Components|Animation|PlayAnimation (Variables|Character|GetMesh) "/Game/RPG_Assets/Npc_RAt/Animation/SM_Rat_Anim_death.SM_Rat_Anim_death" false)
    (Utilities|FlowControl|Sequence
      (:then_0
        (Components|Activation|SetActive (Variables|Character|GetCharacterMovement) false true))
      (:then_1
        (Utilities|FlowControl|Delay 4.0)
        (Audio|Components|Audio|Stop (Variables|Character|GetMesh)))
      (:then_2
        (Utilities|FlowControl|Delay 3.0)
        (Actor|DestroyActor)))))

(fn ConstructionScript)